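; Base AI controller for NPCs that runs a behavior tree and keeps its blackboard fed with data about a target player.
; BeginPlay starts the tree, sets the Player reference by player index and copies AttackRange from the possessed BP_BaseNPC.
; Tick refreshes PlayerLocation regardless of perception.
; Perception updates for FirstPersonCharacter set CanSeePlayer and play a sound on both gain and loss of sensing.
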(event `self.AIPerception.OnTargetPerceptionUpdated`
  (params (Actor :type "Actor Object Reference") (Stimulus :type "AIStimulus Structure"))
  (bind (_age _expirationage _strength _stimuluslocation _receiverlocation _tag _bsuccessfullysensed) (break `AIStimulus` Stimulus))
  ;[1 1 1] Set Blackboard bool CanSeePlayer on Perception Updated
  (cast `/Game/FirstPersonCPP/Blueprints/FirstPersonCharacter` Actor) ; Make sure we sensed the player
  (`BlackboardComponent.SetValueAsBool` (`AIBlueprintHelperLibrary.GetBlackboard` null) "CanSeePlayer" _bsuccessfullysensed) ; Set CanSee true
  ;[1 1 1] Play sound on player detection
  (`GameplayStatics.PlaySoundAtLocation` (`self.Sound`) _receiverlocation (struct) 1.0 1.0 0.0 null null null))

(event `self.ReceiveBeginPlay`
  (`self.RunBehaviorTree` (`self.BehaviourTree`))
  ;[1 1 1] Set blackboard reference for player
  (`self.SetTargetEnemyTeam` (`self.TargetPlayerIndex`))
  ;[1 1 1] Set AttackRange blackboard value
  (bind _asbp_base_npc (cast `/Game/Duality/AI/NPC/BP_BaseNPC` (`self.K2_GetPawn`))
    (:`then`
      (`BlackboardComponent.SetValueAsFloat` (`AIBlueprintHelperLibrary.GetBlackboard` null) "AttackRange" (`/Game/Duality/AI/NPC/BP_BaseNPC.AttackRange` _asbp_base_npc)))
    (:`CastFailed`
      (`KismetSystemLibrary.PrintString` "Cast failed. BaseAIController"))))

(event `self.ReceiveTick`
  (params (DeltaSeconds :type "Float (single-precision)"))
  ;[1 1 1] Set blackboard player location
  (if (`KismetSystemLibrary.IsValid` (`GameplayStatics.GetPlayerController` (`self.TargetPlayerIndex`)))
    (`BlackboardComponent.SetValueAsVector` (`AIBlueprintHelperLibrary.GetBlackboard` null) "PlayerLocation" (`self.K2_GetActorLocation` (`GameplayStatics.GetPlayerCharacter` (`self.TargetPlayerIndex`))))))

(fn `SetTargetEnemyTeam`
  (params (Index :type Integer))
  (set `self.TargetPlayerIndex` Index)
  (`BlackboardComponent.SetValueAsObject` (`AIBlueprintHelperLibrary.GetBlackboard` null) "Player" (`GameplayStatics.GetPlayerCharacter` (`self.TargetPlayerIndex`)))
  (return))

(fn `UserConstructionScript`)