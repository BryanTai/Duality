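; BP_ShootNPC is a ranged NPC that attacks by firing a BP_NPCProjectile at its attack target.
; ExecuteAttack spawns the projectile owned by the NPC, rotated to look at the target's location and always spawned, adjusting for collisions if possible.
; The spawn point adds ProjectileFireLocation's relative location to the actor's location, so the offset ignores actor rotation.
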(event `/Game/Duality/AI/NPC/ICombat.ExecuteAttack`
  (params (AttackTarget :type "Character Object Reference"))
  (bind _returnvalue (+ (.location (`SceneComponent.GetRelativeTransform` (`self.ProjectileFireLocation`))) (.location (`self.GetTransform`))))
  (`|SpawnActorFromClass` "/Game/Duality/Blueprints/BP_NPCProjectile.BP_NPCProjectile_C" (`KismetMathLibrary.MakeTransform` _returnvalue (`KismetMathLibrary.FindLookAtRotation` _returnvalue (`self.K2_GetActorLocation` AttackTarget))) "AdjustIfPossibleButAlwaysSpawn" "OverrideRootScale" self null))

(fn `UserConstructionScript`
  (`parent.UserConstructionScript`))