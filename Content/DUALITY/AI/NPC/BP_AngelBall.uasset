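; BP_AngelBall is an NPC-folder Blueprint that animates three rings, presumably the spinning parts of an angel-like ball.
; On Tick, Ring, Ring1 and Ring2 each add fixed offsets to their own relative rotation on different axes, with Ring1's pitch held at zero.
; The steps ignore delta time, so spin speed depends on frame rate.
; It contains no other active logic.
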(event `self.ReceiveTick`
  (params (DeltaSeconds :type "Float (single-precision)"))
  (bind _ring (`self.Ring`))
  (bind _ring1 (`self.Ring1`))
  (bind _ring2 (`self.Ring2`))
  (bind (_relativerotation_roll _relativerotation_pitch _relativerotation_yaw) (`KismetMathLibrary.BreakRotator` (`SceneComponent.RelativeRotation` _ring1)))
  (bind (_relativerotation_roll_2 _relativerotation_pitch_2 _relativerotation_yaw_2) (`KismetMathLibrary.BreakRotator` (`SceneComponent.RelativeRotation` _ring2)))
  (bind (_relativerotation_roll_3 _relativerotation_pitch_3 _relativerotation_yaw_3) (`KismetMathLibrary.BreakRotator` (`SceneComponent.RelativeRotation` _ring)))
  (`SceneComponent.K2_SetRelativeRotation` _ring2 (`KismetMathLibrary.MakeRotator` _relativerotation_roll_2 (+ _relativerotation_pitch_2 0.3) (+ _relativerotation_yaw_2 0.6)) false false)
  (`SceneComponent.K2_SetRelativeRotation` _ring1 (`KismetMathLibrary.MakeRotator` (+ _relativerotation_roll -0.3) 0.0 (+ _relativerotation_yaw 0.3)) false false)
  (`SceneComponent.K2_SetRelativeRotation` _ring (`KismetMathLibrary.MakeRotator` (+ _relativerotation_roll_3 0.7) (+ _relativerotation_pitch_3 -0.5) _relativerotation_yaw_3) false false))

(fn `UserConstructionScript`)