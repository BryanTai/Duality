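; AI controller for a chase NPC that hunts the first-person player, running the Chase_BT behavior tree on BeginPlay.
; AI Perception updates write whether the player is sensed to the blackboard, along with the last known location while sensed.
; A SetMaxWalkSpeed helper switches the controlled pawn between run and walk speed depending on whether the player is in memory.
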(event `self.AIPerception.OnTargetPerceptionUpdated`
  (params (Actor :type "Actor Object Reference") (Stimulus :type "AIStimulus Structure"))
  (bind (_age _expirationage _strength _stimuluslocation _receiverlocation _tag _bsuccessfullysensed) (break `AIStimulus` Stimulus))
  (cast `/Game/FirstPersonCPP/Blueprints/FirstPersonCharacter` Actor) ; Make sure we sensed the player
  (`BlackboardComponent.SetValueAsBool` (`AIBlueprintHelperLibrary.GetBlackboard` null) "CanSeePlayer" _bsuccessfullysensed) ; Set CanSee true
  (if _bsuccessfullysensed
    (`BlackboardComponent.SetValueAsVector` (`AIBlueprintHelperLibrary.GetBlackboard` null) "PlayerLastKnownLocation" _stimuluslocation) ; If we can see the player, update thier position on the blackboard
  ))

(event `self.ReceiveBeginPlay`
  (`self.RunBehaviorTree` "/Game/Duality/AI/NPC/ChaseAI/Chase_BT.Chase_BT"))

(fn `SetMaxWalkSpeed`
  (params (HasPlayerInMemory :type Boolean))
  (bind _ascharacter_movement_component (cast `CharacterMovementComponent` (`Pawn.GetMovementComponent` (`self.K2_GetPawn`))))
  (if HasPlayerInMemory
    (set `CharacterMovementComponent.MaxWalkSpeed` (`self.RunSpeed`) _ascharacter_movement_component)
    (else
      (set `CharacterMovementComponent.MaxWalkSpeed` (`self.WalkSpeed`) _ascharacter_movement_component))))

(fn `UserConstructionScript`)